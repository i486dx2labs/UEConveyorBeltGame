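; Operator Blueprint for placing a new conveyor belt connector, spawned as a live preview on activation.
; Connector class decides whether ground or wall location is queried; the preview follows it, aligning to wall normals.
; The increase input rotates ground supports in fixed yaw steps, or changes their height with Left Alt held.
; Confirm releases the reference, leaving the connector placed, while Reset destroys any unconfirmed one.
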(event Input|EnhancedActionEvents|EnhancedInputActionIA_Increase
  (params (ActionValue :type Float%20%28double-precision%29) (ElapsedSeconds :type Float%20%28double-precision%29) (TriggeredSeconds :type Float%20%28double-precision%29) (InputAction :type Input%20Action%20Object%20Reference :default "/Game/UserInterface/Input/IA_Increase.IA_Increase"))
  (ConveyorBeltGame|Increase ActionValue))

(fn ConstructionScript
  (|CallParentFunction))

(fn SpawnConnector
  (bind _returnvalue (Game|SpawnActorfromClass (Variables|ConveyorBeltGame|GetConnectorType) (Variables|Default|GetOrigin) "Undefined" "MultiplyWithRoot" 0 0))
  (Variables|ConveyorBeltGame|SetConnector _returnvalue))

(fn OnActivate
  (ConveyorBeltGame|SpawnConnector)
  (|CallParentFunction))

(fn Reset
  (Utilities|FlowControl|Sequence
    (:then_0
      (Utilities|IsValid (Variables|ConveyorBeltGame|GetConnector)
        (:Is%20Valid
          (Actor|DestroyActor (Variables|ConveyorBeltGame|GetConnector)))))
    (:then_1
      (|CallParentFunction))))

(fn Confirm
  (Variables|ConveyorBeltGame|SetConnector 0)
  (|CallParentFunction))

(fn OnGroundLocationChanged
  (params (Location :type Vector :default "0, 0, 0"))
  (|CallParentFunction Location)
  (Transformation|SetActorLocation (Variables|ConveyorBeltGame|GetConnector) Location false false))

(fn OnWallLocationChanged
  (params (Location :type Vector :default "0, 0, 0") (Normal :type Vector :default "0, 0, 0"))
  (|CallParentFunction Location Normal)
  (Transformation|SetActorLocation (Variables|ConveyorBeltGame|GetConnector) Location false false)
  (Transformation|SetActorRotation (Variables|ConveyorBeltGame|GetConnector) (Math|Conversions|RotationFromXVector Normal)))

(fn ShouldQueryGroundLocation
  (Utilities|FlowControl|Sequence
    (:then_0
      (Utilities|IsValid (Variables|ConveyorBeltGame|GetConnector)
        (:Is%20Not%20Valid
          (return false))))
    (:then_1
      (Utilities|Casting|CastToBP_ConveyorBelt_Support_Ground (Variables|ConveyorBeltGame|GetConnector))
      (return true))
    (:then_2
      (Utilities|Casting|CastToBP_ConveyorBelt_Connector_Distributor (Variables|ConveyorBeltGame|GetConnector))
      (return true))
    (:then_3
      (return false))))

(fn ShouldQueryWallLocation
  (Utilities|FlowControl|Sequence
    (:then_0
      (Utilities|IsValid (Variables|ConveyorBeltGame|GetConnector)
        (:Is%20Not%20Valid
          (return false))))
    (:then_1
      (Utilities|Casting|CastToBP_ConveyorBelt_Wall_Mount (Variables|ConveyorBeltGame|GetConnector))
      (return true))
    (:then_2
      (Utilities|Casting|CastToBP_ConveyorBelt_Support_Hatch_In (Variables|ConveyorBeltGame|GetConnector))
      (return true))
    (:then_3
      (Utilities|Casting|CastToBP_ConveyorBelt_Support_Hatch_Out (Variables|ConveyorBeltGame|GetConnector))
      (return true))
    (:then_4
      (return false))))

(fn Rotate
  (params (Step :type Float%20%28double-precision%29))
  (Class|Actor|AddActorWorldRotation (Variables|ConveyorBeltGame|GetConnector) (Math|Rotator|MakeRotator 0.0 0.0 (* Step 45.0))))

(fn IsGroundConnector
  (Utilities|Casting|CastToBP_ConveyorBelt_Support_Ground (Variables|ConveyorBeltGame|GetConnector)
    (:then
      (return true))
    (:CastFailed
      (return false))))

(fn Scale
  (params (Step :type Float%20%28double-precision%29))
  (bind _asbp_conveyor_belt_support_ground (Utilities|Casting|CastToBP_ConveyorBelt_Support_Ground (Variables|ConveyorBeltGame|GetConnector)))
  (Default|IncrementHeight _asbp_conveyor_belt_support_ground (Math|Float|Truncate Step)))

(fn Increase
  (params (Step :type Float%20%28double-precision%29))
  (if (ConveyorBeltGame|IsGroundConnector)
    (if (Game|Player|IsInputKeyDown (Game|GetPlayerController 0) "LeftAlt")
      (ConveyorBeltGame|Scale Step)
      (else
        (ConveyorBeltGame|Rotate Step)))))