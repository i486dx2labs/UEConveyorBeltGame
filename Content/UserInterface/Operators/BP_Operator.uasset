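; BP_Operator is a base actor for interactive operators that the player confirms or cancels through Enhanced Input.
; On BeginPlay it caches the first-person game mode and enables input; cancelling resets, destroys it and notifies the game mode.
; Each tick it queries ground and wall raycasters, gated by check functions that return false by default.
; Reset and the location-change handlers are stubs or debug prints, apparently meant for child operators to override.
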(event Input|EnhancedActionEvents|EnhancedInputActionIA_Confirm
  (params (ActionValue :type Boolean) (ElapsedSeconds :type Float%20%28double-precision%29) (TriggeredSeconds :type Float%20%28double-precision%29) (InputAction :type Input%20Action%20Object%20Reference :default "/Game/UserInterface/Input/IA_Confirm.IA_Confirm"))
  (:Completed
    (ConveyorBeltGame|Confirm)))

(event Input|EnhancedActionEvents|EnhancedInputActionIA_Cancel
  (params (ActionValue :type Boolean) (ElapsedSeconds :type Float%20%28double-precision%29) (TriggeredSeconds :type Float%20%28double-precision%29) (InputAction :type Input%20Action%20Object%20Reference :default "/Game/UserInterface/Input/IA_Cancel.IA_Cancel"))
  (:Completed
    (ConveyorBeltGame|Cancel)))

(event EventTick
  (params (DeltaSeconds :type Float%20%28single-precision%29))
  (ConveyorBeltGame|TickRaycasters))

(event EventBeginPlay
  (ConveyorBeltGame|OnActivate))

(fn ConstructionScript)

(fn OnActivate
  (Utilities|FlowControl|Sequence
    (:then_0
      (ConveyorBeltGame|FindGameMode)
      (Input|EnableInput (Game|GetPlayerController 0)))
    (:then_1
      (Development|PrintText (Utilities|Text|FormatText "Activating operator: {operator}" (Utilities|GetClassDisplayName (Utilities|GetClass self)))))))

(fn FindGameMode
  (bind _asbp_first_person_game_mode (Utilities|Casting|CastToBP_FirstPersonGameMode (Game|GetGameMode)))
  (Variables|ConveyorBeltGame|References|SetGameMode _asbp_first_person_game_mode))

(fn TickRaycasters
  (Utilities|FlowControl|Sequence
    (:then_0
      (if (ConveyorBeltGame|ShouldQueryGroundLocation)
        (Default|Query (Variables|Default|GetGround%20Raycaster) self)))
    (:then_1
      (if (ConveyorBeltGame|ShouldQueryWallLocation)
        (Default|Query (Variables|Default|GetWall%20Raycaster) self)))))

(fn Confirm
  (ConveyorBeltGame|Reset))

(fn Cancel
  (Utilities|FlowControl|Sequence
    (:then_0
      (ConveyorBeltGame|Reset))
    (:then_1
      (Actor|DestroyActor))
    (:then_2
      (Default|NotifyOperatorCanceled (Variables|ConveyorBeltGame|References|GetGameMode)))))

(fn Reset)

(fn OnGroundLocationChanged
  (params (Location :type Vector))
  (Development|PrintString (Utilities|String|ToString(Vector) Location)))

(fn OnWallLocationChanged
  (params (Location :type Vector) (Normal :type Vector)))

(fn ShouldQueryGroundLocation
  (return false))

(fn ShouldQueryWallLocation
  (return false))