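; AC_Raycaster is a raycaster component that defines a camera-based trace segment for player 0.
; GetTraceStart returns the camera manager's location, and GetTraceEnd offsets that point along the camera manager actor's forward vector by Distance.
; Query takes an Operator but has an empty body, so no trace is performed here.
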(fn Query
  (params (Operator :type BP%20Operator%20Object%20Reference)))

(fn GetTraceStart
  (return (Camera|GetCameraLocation (Variables|/Script/Engine.PlayerController|GetPlayerCameraManager (Game|GetPlayerController 0)))))

(fn GetTraceEnd
  (return (+ (ConveyorBeltGame|GetTraceStart) (* (Transformation|GetActorForwardVector (Variables|/Script/Engine.PlayerController|GetPlayerCameraManager (Game|GetPlayerController 0))) (Variables|ConveyorBeltGame|GetDistance)))))