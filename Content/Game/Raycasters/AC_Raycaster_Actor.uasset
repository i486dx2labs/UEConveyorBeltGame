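; AC_Raycaster_Actor is a raycaster that finds the actor along a trace and reports hover results to an operator.
; Query runs the parent query, then line traces on the Camera channel between the trace start and end points.
; A hit passes the actor and hit result to HandleActorHit, an empty stub here, while a miss tells the operator nothing is hovered.
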(fn Query
  (params (Operator :type BP%20Operator%20Object%20Reference))
  (|CallParentFunction Operator)
  (bind (_outhit _returnvalue) (Collision|LineTraceByChannel (CallFunction|GetTraceStart) (CallFunction|GetTraceEnd) "TraceTypeQuery2" false 0 "None"))
  (LocalVariables|SetHit _outhit)
  (if _returnvalue
    (ConveyorBeltGame|HandleActorHit Operator (.HitActor (Collision|BreakHitResult (LocalVariables|GetHit))) (LocalVariables|GetHit))
    (else
      (ConveyorBeltGame|HandleEmptyHit Operator))))

(fn HandleActorHit
  (params (Operator :type BP%20Operator%20Object%20Reference) (Actor :type Actor%20Object%20Reference) (Hit :type Hit%20Result%20Structure)))

(fn HandleEmptyHit
  (params (Operator :type BP%20Operator%20Object%20Reference))
  (Default|OnNothingHovered Operator))