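; Base raycaster component that traces against level-structure object types, with child raycasters expected to supply the hit rules.
; Query runs the parent query, line-traces, and optionally snaps the hit location to a grid when the Controller enables snapping.
; It skips locations unchanged within tolerance or with invalid normals, then caches the location and calls PublishHit.
; IsValidNormal (false by default) and the empty PublishHit act as override hooks.
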(fn Query
  (params (Operator :type BP%20Operator%20Object%20Reference))
  (|CallParentFunction Operator)
  (bind (_outhit _returnvalue) (Collision|LineTraceForObjects (CallFunction|GetTraceStart) (CallFunction|GetTraceEnd) (Variables|ConveyorBeltGame|GetLevelObjectTypes) false 0 "None"))
  (LocalVariables|SetHit _outhit)
  (if _returnvalue
    (Utilities|FlowControl|Sequence
      (:then_0
        (bind _location (ConveyorBeltGame|ExtractHitLocation (LocalVariables|GetHit)))
        (LocalVariables|SetLocation _location))
      (:then_1
        (if (Utilities|Operators|EqualEqual (LocalVariables|GetLocation) (Variables|ConveyorBeltGame|GetPreviousLocation) (Variables|Default|GetErrorTolerance))
          (return)
          (elif (not (ConveyorBeltGame|IsValidNormal (.Normal (Collision|BreakHitResult (LocalVariables|GetHit)))))
            (return))))
      (:then_2
        (bind _output_get (Variables|ConveyorBeltGame|SetPreviousLocation (LocalVariables|GetLocation)))
        (ConveyorBeltGame|PublishHit Operator (LocalVariables|GetHit) _output_get)))))

(fn IsValidNormal
  (params (Normal :type Vector))
  (return false))

(fn PublishHit
  (params (Operator :type BP%20Operator%20Object%20Reference) (Hit :type Hit%20Result%20Structure) (ActualLocation :type Vector)))

(fn ExtractHitLocation
  (params (Hit :type Hit%20Result%20Structure))
  (LocalVariables|SetHitLocation (.Location (Collision|BreakHitResult Hit)))
  (if (Variables|/Game/FirstPerson/Blueprints/BP_FirstPersonPlayerController.BP_FirstPersonPlayerController_C|GetbGridSnapEnabled (Variables|Default|GetController))
    (return (Class|KismetMathLibrary|VectorSnappedtoGrid (LocalVariables|GetHitLocation) 5e+01))
    (else
      (return (LocalVariables|GetHitLocation)))))