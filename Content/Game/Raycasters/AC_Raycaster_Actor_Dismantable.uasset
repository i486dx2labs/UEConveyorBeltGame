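; Actor raycaster component that, judging by its name, targets dismantlable objects, with special handling for conveyor belt connectors.
; Its hit handler runs the parent logic, then notifies the Operator through OnConnectorHovered when the hit actor is a ConveyorBeltConnector.
; A Sequence with an early return acts as a fallback: any other actor is passed on to empty-hit handling.
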(event EventBeginPlay
  (|CallParentFunction) ; This node is disabled and will not be called.\nDrag off pins to build functionality.
)

(event EventTick
  (params (DeltaSeconds :type Float%20%28single-precision%29)))

(fn HandleActorHit
  (params (Operator :type BP%20Operator%20Object%20Reference) (Actor :type Actor%20Object%20Reference) (Hit :type Hit%20Result%20Structure))
  (|CallParentFunction Operator Actor Hit)
  (Utilities|FlowControl|Sequence
    (:then_0
      (bind _asconveyor_belt_connector (Utilities|Casting|CastToConveyorBeltConnector Actor))
      (Default|OnConnectorHovered Operator _asconveyor_belt_connector)
      (return))
    (:then_1
      (CallFunction|HandleEmptyHit Operator))))