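; Raycaster component that finds which conveyor belt connector or socket an Operator is hovering, filtered by a configurable list of selection target types.
; Each query line-traces on the Camera channel and tests the hit in order: connector, ground-placeable connector, available input socket, available output socket.
; Sockets are resolved from the hit component's attach parent.
; The first match is reported through the Operator's hover callback; otherwise it reports nothing hovered.
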(fn Query
  (params (Operator :type BP%20Operator%20Object%20Reference))
  (|CallParentFunction Operator)
  (bind (_outhit _returnvalue) (Collision|LineTraceByChannel (CallFunction|GetTraceStart) (CallFunction|GetTraceEnd) "TraceTypeQuery2" false 0 "None"))
  (LocalVariables|SetHit _outhit)
  (if _returnvalue
    (ConveyorBeltGame|HandleActorHit Operator (.HitActor (Collision|BreakHitResult (LocalVariables|GetHit))) (LocalVariables|GetHit))
    (else
      (ConveyorBeltGame|HandleEmptyHit Operator))))

(fn HandleActorHit
  (params (Operator :type BP%20Operator%20Object%20Reference) (Actor :type Actor%20Object%20Reference) (Hit :type Hit%20Result%20Structure))
  (Utilities|FlowControl|Sequence
    (:then_0
      (LocalVariables|SetHitComponent (.HitComponent (Collision|BreakHitResult Hit))))
    (:then_1
      (bind _handled (ConveyorBeltGame|HandleConnectorTarget Operator Actor))
      (if _handled
        (return)))
    (:then_2
      (bind _handled_2 (ConveyorBeltGame|HandleGroundConnectorTarget Operator Actor))
      (if _handled_2
        (return)))
    (:then_3
      (bind _handled_3 (ConveyorBeltGame|HandleInputSocketTarget Operator Actor Hit))
      (if _handled_3
        (return)))
    (:then_4
      (bind _handled_4 (ConveyorBeltGame|HandleOutputSocketTarget Operator Actor Hit))
      (if _handled_4
        (return)))
    (:then_5
      (ConveyorBeltGame|HandleEmptyHit Operator))))

(fn HandleEmptyHit
  (params (Operator :type BP%20Operator%20Object%20Reference))
  (Default|OnNothingHovered Operator))

(fn SetTargets
  (params (Targets :type Set%20of%20E_SelectionTarget%20Enums :default "NewEnumerator0"))
  (Variables|ConveyorBeltGame|SetTargets Targets))

(fn HandleConnectorTarget
  (params (Operator :type BP%20Operator%20Object%20Reference) (Actor :type Actor%20Object%20Reference))
  (Utilities|HasSelectionTarget "NewEnumerator0"
    (:Yes
      (bind _asconveyor_belt_connector (Utilities|Casting|CastToConveyorBeltConnector Actor))
      (Default|OnConnectorHovered Operator _asconveyor_belt_connector)
      (return true))))

(fn HandleGroundConnectorTarget
  (params (Operator :type BP%20Operator%20Object%20Reference) (Actor :type Actor%20Object%20Reference))
  (Utilities|HasSelectionTarget "NewEnumerator1"
    (:Yes
      (bind _asconveyor_belt_connector (Utilities|Casting|CastToConveyorBeltConnector Actor))
      (if (Variables|/Script/ConveyorBeltSystem.ConveyorBeltConnector|GetbCanPlaceOnGround _asconveyor_belt_connector)
        (Default|OnConnectorHovered Operator _asconveyor_belt_connector)
        (return true)))))

(fn HandleInputSocketTarget
  (params (Operator :type BP%20Operator%20Object%20Reference) (Actor :type Actor%20Object%20Reference) (Hit :type Hit%20Result%20Structure))
  (Utilities|HasSelectionTarget "NewEnumerator3"
    (:Yes
      (bind _socket (Utilities|IsSocketComponent Hit true)
        (:Yes
          (Default|OnSocketHovered Operator _socket)
          (return true))))))

(fn HandleOutputSocketTarget
  (params (Operator :type BP%20Operator%20Object%20Reference) (Actor :type Actor%20Object%20Reference) (Hit :type Hit%20Result%20Structure))
  (Utilities|HasSelectionTarget "NewEnumerator6"
    (:Yes
      (bind _socket (Utilities|IsSocketComponent Hit false)
        (:Yes
          (Default|OnSocketHovered Operator _socket)
          (return true))))))