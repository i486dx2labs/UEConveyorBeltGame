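; BP_Operator_Connector_Clone is a build operator that duplicates an existing connector.
; It queries a cloneable raycaster on tick and tints the hovered connector with a hologram material, restoring it on reset or when nothing is hovered.
; Confirm spawns a same-class copy at the same transform, copying height for conveyor ground supports.
; It then activates a new Connector Add operator through the GameMode, passing it the clone.
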(fn ConstructionScript
  (|CallParentFunction))

(fn TickRaycasters
  (|CallParentFunction)
  (Default|Query (Variables|Default|GetCloneableRaycaster) self))

(fn OnConnectorHovered
  (params (Connector :type Conveyor%20Belt%20Connector%20Object%20Reference))
  (Utilities|FlowControl|Sequence
    (:then_0
      (CallFunction|Reset))
    (:then_1
      (bind _output_get (Variables|ConveyorBeltGame|References|SetLastHoveredConnector Connector))
      (Class|ConveyorBeltConnector|ApplyMaterial _output_get "/ConveyorBeltSystem/Materials/MI_ConveyorBelt_Hologram_Translucent_Info.MI_ConveyorBelt_Hologram_Translucent_Info"))
    (:then_2
      (|CallParentFunction Connector))))

(fn OnNothingHovered
  (|CallParentFunction)
  (CallFunction|Reset))

(fn Reset
  (Utilities|FlowControl|Sequence
    (:then_0
      (Utilities|IsValid (Variables|ConveyorBeltGame|References|GetLastHoveredConnector)
        (:Is%20Valid
          (Class|ConveyorBeltConnector|RestoreOriginalMaterial (Variables|ConveyorBeltGame|References|GetLastHoveredConnector))
          (Variables|ConveyorBeltGame|References|SetLastHoveredConnector 0))))
    (:then_1
      (|CallParentFunction))))

(fn Confirm
  (Utilities|FlowControl|Sequence
    (:then_0
      (Utilities|IsValid (Variables|ConveyorBeltGame|References|GetLastHoveredConnector)
        (:Is%20Valid
          (bind _returnvalue (Game|SpawnActorfromClass (Utilities|GetClass (Variables|ConveyorBeltGame|References|GetLastHoveredConnector)) (Transformation|GetActorTransform (Variables|ConveyorBeltGame|References|GetLastHoveredConnector)) "AlwaysSpawn" "MultiplyWithRoot" 0 0))
          (LocalVariables|SetClone _returnvalue))))
    (:then_1
      (bind _asbp_conveyor_belt_support_ground (Utilities|Casting|CastToBP_ConveyorBelt_Support_Ground (Variables|ConveyorBeltGame|References|GetLastHoveredConnector)))
      (bind _asbp_conveyor_belt_support_ground_2 (Utilities|Casting|CastToBP_ConveyorBelt_Support_Ground (LocalVariables|GetClone)))
      (Default|SetHeight _asbp_conveyor_belt_support_ground_2 (Variables|/ConveyorBeltSystem/Blueprints/Connectors/BP_ConveyorBelt_Support_Ground.BP_ConveyorBelt_Support_Ground_C|GetHeight _asbp_conveyor_belt_support_ground)))
    (:then_2
      (bind _returnvalue_2 (Game|SpawnActorfromClass "/Game/Game/Operators/BP_Operator_Connector_Add.BP_Operator_Connector_Add_C" (Variables|Default|GetOrigin) "Undefined" "MultiplyWithRoot" 0 0 (LocalVariables|GetClone) 0))
      (Default|ActivateOperator (Variables|Default|GetGameMode) _returnvalue_2)
      (|CallParentFunction))))