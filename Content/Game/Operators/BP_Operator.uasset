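; Base actor for player-driven conveyor belt operators, handling target hover, selection, confirm and cancel.
; While selection targets are set, a raycaster queries each tick, and hover handlers track connectors and sockets, highlighting connectors with a hologram material.
; Confirm commits the focused target or, outside selection mode, follows ConfirmBehavior to reset, cancel, reactivate or restore the default operator via the game mode.
; Cancel resets, notifies the game mode and destroys the actor.
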(event Input|EnhancedActionEvents|EnhancedInputActionIA_Confirm
  (params (ActionValue :type Boolean) (ElapsedSeconds :type Float%20%28double-precision%29) (TriggeredSeconds :type Float%20%28double-precision%29) (InputAction :type Input%20Action%20Object%20Reference :default "/Game/Game/Input/IA_Confirm.IA_Confirm"))
  (:Completed
    (ConveyorBeltGame|Confirmation|Confirm)))

(event Input|EnhancedActionEvents|EnhancedInputActionIA_Cancel
  (params (ActionValue :type Boolean) (ElapsedSeconds :type Float%20%28double-precision%29) (TriggeredSeconds :type Float%20%28double-precision%29) (InputAction :type Input%20Action%20Object%20Reference :default "/Game/Game/Input/IA_Cancel.IA_Cancel"))
  (:Completed
    (ConveyorBeltGame|Cancel)))

(event EventBeginPlay
  (ConveyorBeltGame|FindGameMode))

(event EventTick
  (params (DeltaSeconds :type Float%20%28single-precision%29))
  (ConveyorBeltGame|TickRaycasters))

(fn ConstructionScript)

(fn OnActivate
  (Variables|Default|SetManager (Class|ConveyorBeltUtility|FindConveyorBeltManager self))
  (Input|EnableInput (Game|GetPlayerController 0))
  (ConveyorBeltGame|Log "Activating"))

(fn FindGameMode
  (bind _asbp_first_person_game_mode (Utilities|Casting|CastToBP_FirstPersonGameMode (Game|GetGameMode)))
  (Variables|ConveyorBeltGame|References|SetGameMode _asbp_first_person_game_mode))

(fn TickRaycasters
  (if (ConveyorBeltGame|Selection|IsSelectionModeActive)
    (Default|Query (Variables|Default|GetSelectionTargetRaycaster) self)))

(fn Confirm
  (if (ConveyorBeltGame|Selection|IsSelectionModeActive)
    (ConveyorBeltGame|Confirmation|ConfirmSelection)
    (else
      (ConveyorBeltGame|Confirmation|ConfirmOperation))))

(fn Cancel
  (ConveyorBeltGame|Log "Canceling")
  (Utilities|FlowControl|Sequence
    (:then_0
      (ConveyorBeltGame|Reset))
    (:then_1
      (Default|NotifyOperatorCanceled (Variables|ConveyorBeltGame|References|GetGameMode)))
    (:then_2
      (Actor|DestroyActor))))

(fn Reset
  (ConveyorBeltGame|Log "Resetting")
  (Utilities|FlowControl|Sequence
    (:then_0
      (Utilities|IsValid (Variables|ConveyorBeltGame|References|GetSelectedConnector)
        (:Is%20Valid
          (Class|ConveyorBeltConnector|ApplyMaterialTheme (Variables|ConveyorBeltGame|References|GetSelectedConnector))
          (Variables|ConveyorBeltGame|References|SetSelectedConnector 0))))
    (:then_1
      (Utilities|IsValid (Variables|ConveyorBeltGame|References|GetSelectedSocket)
        (:Is%20Valid
          (Variables|ConveyorBeltGame|References|SetSelectedSocket 0))))
    (:then_2
      (ConveyorBeltGame|Selection|OnNothingHovered))))

(fn OnGroundLocationChanged
  (params (Location :type Vector)))

(fn OnWallLocationChanged
  (params (Location :type Vector) (Normal :type Vector)))

(fn OnConnectorHovered
  (params (Connector :type Conveyor%20Belt%20Connector%20Object%20Reference))
  (if (not (== Connector (Variables|ConveyorBeltGame|References|GetFocusedConnector)))
    (Utilities|FlowControl|Sequence
      (:then_0
        (Utilities|IsValid (Variables|ConveyorBeltGame|References|GetFocusedConnector)
          (:Is%20Valid
            (ConveyorBeltGame|Selection|OnConnectorMouseExit (Variables|ConveyorBeltGame|References|GetFocusedConnector)))))
      (:then_1
        (ConveyorBeltGame|Selection|OnConnectorMouseEnter Connector)))))

(fn OnConnectorMouseEnter
  (params (Connector :type Conveyor%20Belt%20Connector%20Object%20Reference))
  (bind _output_get (Variables|ConveyorBeltGame|References|SetFocusedConnector Connector))
  (Class|ConveyorBeltConnector|ApplyMaterial _output_get "/ConveyorBeltSystem/Materials/MI_ConveyorBelt_Hologram_Translucent_Info.MI_ConveyorBelt_Hologram_Translucent_Info")
  (ConveyorBeltGame|Log (Utilities|Text|FormatText "OnConnectorMouseEnter: {connector}" (Utilities|GetDisplayName Connector))))

(fn OnConnectorMouseExit
  (params (Connector :type Conveyor%20Belt%20Connector%20Object%20Reference))
  (Class|ConveyorBeltConnector|ApplyMaterialTheme Connector)
  (Variables|ConveyorBeltGame|References|SetFocusedConnector 0)
  (ConveyorBeltGame|Log (Utilities|Text|FormatText "OnConnectorMouseExit: {connector}" (Utilities|GetDisplayName Connector))))

(fn OnConnectorSelected
  (params (Connector :type Conveyor%20Belt%20Connector%20Object%20Reference))
  (Variables|ConveyorBeltGame|References|SetSelectedConnector Connector)
  (Development|PrintText (Utilities|Text|FormatText "OnConnectorSelected: {connector}" (Utilities|GetDisplayName Connector))))

(fn OnNothingHovered
  (Utilities|FlowControl|Sequence
    (:then_0
      (Utilities|IsValid (Variables|ConveyorBeltGame|References|GetFocusedConnector)
        (:Is%20Valid
          (ConveyorBeltGame|Selection|OnConnectorMouseExit (Variables|ConveyorBeltGame|References|GetFocusedConnector)))))
    (:then_1
      (Utilities|IsValid (Variables|ConveyorBeltGame|References|GetFocusedSocket)
        (:Is%20Valid
          (ConveyorBeltGame|Selection|OnSocketMouseExit (Variables|ConveyorBeltGame|References|GetFocusedSocket)))))))

(fn EnterSelectionMode
  (params (Targets :type Set%20of%20E_SelectionTarget%20Enums :default "NewEnumerator0"))
  (Variables|/Game/Game/Raycasters/AC_Raycaster_SelectionTarget.AC_Raycaster_SelectionTarget_C|SetTargets (Variables|Default|GetSelectionTargetRaycaster) Targets))

(fn ExitSelectionMode
  (Utilities|Set|Clear (Variables|/Game/Game/Raycasters/AC_Raycaster_SelectionTarget.AC_Raycaster_SelectionTarget_C|GetTargets (Variables|Default|GetSelectionTargetRaycaster))))

(fn IsSelectionModeActive
  (return (Utilities|Set|IsNotEmpty (Variables|/Game/Game/Raycasters/AC_Raycaster_SelectionTarget.AC_Raycaster_SelectionTarget_C|GetTargets (Variables|Default|GetSelectionTargetRaycaster)))))

(fn ConfirmSelection
  (ConveyorBeltGame|Log "Confirming selection")
  (ConveyorBeltGame|Selection|ExitSelectionMode)
  (Utilities|FlowControl|Sequence
    (:then_0
      (Utilities|IsValid (Variables|ConveyorBeltGame|References|GetFocusedConnector)
        (:Is%20Valid
          (ConveyorBeltGame|Selection|OnConnectorSelected (Variables|ConveyorBeltGame|References|GetFocusedConnector)))))
    (:then_1
      (Utilities|IsValid (Variables|ConveyorBeltGame|References|GetFocusedSocket)
        (:Is%20Valid
          (ConveyorBeltGame|Selection|OnSocketSelected (Variables|ConveyorBeltGame|References|GetFocusedSocket)))))))

(fn HasSelectedTarget
  (return (or (Utilities|IsValid (Variables|ConveyorBeltGame|References|GetSelectedConnector)) false)))

(fn OnSocketHovered
  (params (Socket :type Conveyor%20Belt%20Socket%20Object%20Reference))
  (if (not (== Socket (Variables|ConveyorBeltGame|References|GetFocusedSocket)))
    (Utilities|FlowControl|Sequence
      (:then_0
        (Utilities|IsValid (Variables|ConveyorBeltGame|References|GetFocusedSocket)
          (:Is%20Valid
            (ConveyorBeltGame|Selection|OnSocketMouseExit (Variables|ConveyorBeltGame|References|GetFocusedSocket)))))
      (:then_1
        (ConveyorBeltGame|Selection|OnSocketMouseEnter Socket)))))

(fn OnSocketMouseEnter
  (params (Socket :type Conveyor%20Belt%20Socket%20Object%20Reference))
  (bind _output_get (Variables|ConveyorBeltGame|References|SetFocusedSocket Socket))
  (ConveyorBeltGame|Log (Utilities|Text|FormatText "OnSocketMouseEnter: {socket}" (Utilities|GetDisplayName _output_get))))

(fn OnSocketMouseExit
  (params (Socket :type Conveyor%20Belt%20Socket%20Object%20Reference))
  (Variables|ConveyorBeltGame|References|SetFocusedSocket 0)
  (ConveyorBeltGame|Log (Utilities|Text|FormatText "OnSocketMouseExit: {socket}" (Utilities|GetDisplayName Socket))))

(fn OnSocketSelected
  (params (Socket :type Conveyor%20Belt%20Socket%20Object%20Reference))
  (bind _output_get (Variables|ConveyorBeltGame|References|SetSelectedSocket Socket))
  (ConveyorBeltGame|Log (Utilities|Text|FormatText "OnSocketSelected: {socket}" (Utilities|GetDisplayName _output_get))))

(fn Log
  (params (Message :type Text))
  (Development|PrintText (Utilities|Text|FormatText "[{operator}] {message}" (Utilities|GetClassDisplayName (Utilities|GetClass self)) Message)))

(fn ConfirmOperation
  (ConveyorBeltGame|Log "Confirming operation")
  (switch Utilities|FlowControl|Switch|SwitchonE_Operator_ConfirmBehavior (Variables|ConveyorBeltGame|Settings|GetConfirmBehavior)
    (:NewEnumerator1
      (ConveyorBeltGame|Reset))
    (:NewEnumerator2
      (ConveyorBeltGame|Cancel))
    (:NewEnumerator3
      (Default|ActivateOperatorbyType (Variables|ConveyorBeltGame|References|GetGameMode) (Utilities|GetClass self)))
    (:NewEnumerator6
      (Default|ActivateDefaultOperator (Variables|ConveyorBeltGame|References|GetGameMode)))))