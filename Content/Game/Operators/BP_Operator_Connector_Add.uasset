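; Placement operator that spawns a new connector as a collision-free, themed preview following the ground or wall surface.
; The connector's ground flag picks which raycaster runs; wall connectors align to the surface normal, while increase/decrease input yaws ground connectors in fixed steps.
; Confirm restores collision and hands the connector to a newly activated BP_Operator_Connector_Offset, while Reset destroys the unconfirmed one.
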(event Input|EnhancedActionEvents|EnhancedInputActionIA_Increase
  (params (ActionValue :type Boolean) (ElapsedSeconds :type Float%20%28double-precision%29) (TriggeredSeconds :type Float%20%28double-precision%29) (InputAction :type Input%20Action%20Object%20Reference :default "/Game/Game/Input/IA_Increase.IA_Increase"))
  (ConveyorBeltGame|Increase 1.0))

(event Input|EnhancedActionEvents|EnhancedInputActionIA_Decrease
  (params (ActionValue :type Boolean) (ElapsedSeconds :type Float%20%28double-precision%29) (TriggeredSeconds :type Float%20%28double-precision%29) (InputAction :type Input%20Action%20Object%20Reference :default "/Game/Game/Input/IA_Decrease.IA_Decrease"))
  (ConveyorBeltGame|Increase -1.0))

(fn ConstructionScript
  (|CallParentFunction))

(fn SpawnConnector
  (Utilities|FlowControl|Sequence
    (:then_0
      (Utilities|IsValid (Variables|ConveyorBeltGame|GetConnector)
        (:Is%20Not%20Valid
          (bind _returnvalue (Game|SpawnActorfromClass (Variables|ConveyorBeltGame|GetConnectorType) (Variables|Default|GetOrigin) "Undefined" "MultiplyWithRoot" 0 0))
          (Variables|ConveyorBeltGame|SetConnector _returnvalue))))
    (:then_1
      (Class|ConveyorBeltConnector|ApplyCollisionMode (Variables|ConveyorBeltGame|GetConnector) "NoCollision")
      (Variables|/Script/ConveyorBeltSystem.ConveyorBeltConnector|SetMaterialTheme (Variables|ConveyorBeltGame|GetConnector) (Default|GetCurrentMaterialTheme (Variables|Default|GetGameMode)))
      (Class|ConveyorBeltConnector|ApplyMaterialTheme (Variables|ConveyorBeltGame|GetConnector)))))

(fn OnActivate
  (Utilities|FlowControl|Sequence
    (:then_0
      (ConveyorBeltGame|SpawnConnector))
    (:then_1
      (|CallParentFunction))))

(fn Reset
  (Utilities|FlowControl|Sequence
    (:then_0
      (Utilities|IsValid (Variables|ConveyorBeltGame|GetConnector)
        (:Is%20Valid
          (Actor|DestroyActor (Variables|ConveyorBeltGame|GetConnector)))))
    (:then_1
      (|CallParentFunction))))

(fn Confirm
  (Utilities|FlowControl|Sequence
    (:then_0
      (Utilities|IsValid (Variables|ConveyorBeltGame|GetConnector)
        (:Is%20Valid
          (Class|ConveyorBeltConnector|ApplyCollisionMode (Variables|ConveyorBeltGame|GetConnector) "QueryAndPhysics"))))
    (:then_1
      (bind _returnvalue (Game|SpawnActorfromClass "/Game/Game/Operators/BP_Operator_Connector_Offset.BP_Operator_Connector_Offset_C" (Variables|Default|GetOrigin) "Undefined" "MultiplyWithRoot" 0 (Variables|ConveyorBeltGame|GetConnector) 0))
      (LocalVariables|SetNextOperator _returnvalue)
      (Variables|ConveyorBeltGame|SetConnector 0)
      (|CallParentFunction))
    (:then_2
      (Default|ActivateOperator (Variables|Default|GetGameMode) (LocalVariables|GetNextOperator)))))

(fn OnGroundLocationChanged
  (params (Location :type Vector :default "0, 0, 0"))
  (|CallParentFunction Location)
  (Transformation|SetActorLocation (Variables|ConveyorBeltGame|GetConnector) Location false false))

(fn OnWallLocationChanged
  (params (Location :type Vector :default "0, 0, 0") (Normal :type Vector :default "0, 0, 0"))
  (|CallParentFunction Location Normal)
  (Transformation|SetActorLocation (Variables|ConveyorBeltGame|GetConnector) Location false false)
  (Transformation|SetActorRotation (Variables|ConveyorBeltGame|GetConnector) (Math|Conversions|RotationFromXVector Normal)))

(fn ShouldQueryGroundLocation
  (return (ConveyorBeltGame|IsGroundConnector)))

(fn ShouldQueryWallLocation
  (return (not (ConveyorBeltGame|IsGroundConnector))))

(fn Rotate
  (params (Step :type Float%20%28double-precision%29))
  (Class|Actor|AddActorWorldRotation (Variables|ConveyorBeltGame|GetConnector) (Math|Rotator|MakeRotator 0.0 0.0 (* Step 45.0))))

(fn IsGroundConnector
  (Utilities|IsValid (Variables|ConveyorBeltGame|GetConnector)
    (:Is%20Valid
      (return (Variables|/Script/ConveyorBeltSystem.ConveyorBeltConnector|GetbCanPlaceOnGround (Variables|ConveyorBeltGame|GetConnector))))
    (:Is%20Not%20Valid
      (return false))))

(fn Increase
  (params (Step :type Float%20%28double-precision%29))
  (Utilities|IsValid (Variables|ConveyorBeltGame|GetConnector)
    (:Is%20Valid
      (if (ConveyorBeltGame|IsGroundConnector)
        (ConveyorBeltGame|Rotate Step)))))

(fn TickRaycasters
  (|CallParentFunction)
  (Utilities|FlowControl|Sequence
    (:then_0
      (if (ConveyorBeltGame|ShouldQueryGroundLocation)
        (Default|Query (Variables|Default|GetGroundRaycaster) self)))
    (:then_1
      (if (ConveyorBeltGame|ShouldQueryWallLocation)
        (Default|Query (Variables|Default|GetWallRaycaster) self)))))