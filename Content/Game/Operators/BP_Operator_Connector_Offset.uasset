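; BP_Operator_Connector_Offset is an operator that adjusts the offset of a selected connector.
; On activation it enters selection mode with its targets if no valid connector is selected, then runs the parent activation either way.
; Completed Enhanced Input increase and decrease actions feed a shared ChangeOffset function, which steps the selected connector's offset up or down by one whole unit when that connector is valid.
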(event Input|EnhancedActionEvents|EnhancedInputActionIA_Increase
  (params (ActionValue :type Boolean) (ElapsedSeconds :type Float%20%28double-precision%29) (TriggeredSeconds :type Float%20%28double-precision%29) (InputAction :type Input%20Action%20Object%20Reference :default "/Game/Game/Input/IA_Increase.IA_Increase"))
  (:Completed
    (ConveyorBeltGame|ChangeOffset 1.0)))

(event Input|EnhancedActionEvents|EnhancedInputActionIA_Decrease
  (params (ActionValue :type Boolean) (ElapsedSeconds :type Float%20%28double-precision%29) (TriggeredSeconds :type Float%20%28double-precision%29) (InputAction :type Input%20Action%20Object%20Reference :default "/Game/Game/Input/IA_Decrease.IA_Decrease"))
  (:Completed
    (ConveyorBeltGame|ChangeOffset -1.0)))

(fn ConstructionScript
  (|CallParentFunction))

(fn ChangeOffset
  (params (Step :type Float%20%28double-precision%29))
  (Utilities|IsValid (Variables|Default|GetSelectedConnector)
    (:Is%20Valid
      (Class|ConveyorBeltConnector|IncrementOffset (Variables|Default|GetSelectedConnector) (Math|Float|Truncate Step)))))

(fn OnActivate
  (Utilities|IsValid (Variables|Default|GetSelectedConnector)
    (:Is%20Valid
      (|CallParentFunction))
    (:Is%20Not%20Valid
      (CallFunction|EnterSelectionMode (LocalVariables|GetTargets))
      (|CallParentFunction))))