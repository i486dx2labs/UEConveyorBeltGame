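; Belt-building operator that starts a conveyor belt from a selected input socket.
; Activation enters target selection mode; selecting an input spawns a short ground support in front of it, using only the socket's X/Y position, if available and no connector exists.
; The conveyor belt manager builds an unaccepted belt between that socket and the connector's output.
; Reset destroys the belt but leaves the connector.
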(fn ConstructionScript
  (|CallParentFunction))

(fn OnActivate
  (CallFunction|EnterSelectionMode (LocalVariables|GetTargets))
  (|CallParentFunction))

(fn OnSocketSelected
  (params (Socket :type Conveyor%20Belt%20Socket%20Object%20Reference))
  (|CallParentFunction Socket)
  (if (Variables|/Script/ConveyorBeltSystem.ConveyorBeltSocket|GetbIsInput Socket)
    (CallFunction|SpawnConnector)
    (ConveyorBeltGame|SpawnBelt Socket)))

(fn SpawnBelt
  (params (InputSocket :type Conveyor%20Belt%20Socket%20Object%20Reference))
  (bind _returnvalue (Class|ConveyorBeltManager|BuildOneShotUsingSockets (Class|ConveyorBeltUtility|FindConveyorBeltManager self) InputSocket (Class|ConveyorBeltConnector|GetSingleOutputSocket (Variables|Default|GetConnector) true) "/ConveyorBeltSystem/Blueprints/Belts/BP_ConveyorBelt_01.BP_ConveyorBelt_01_C" false false))
  (Variables|ConveyorBeltGame|References|SetSpawnedBelt _returnvalue))

(fn SpawnConnectorinFrontOfSocket
  (params (InputSocket :type Conveyor%20Belt%20Socket%20Object%20Reference))
  (Utilities|FlowControl|Sequence
    (:then_0
      (LocalVariables|SetConnectorLocation (+ (Transformation|GetWorldLocation InputSocket) (* (Math|Vector|GetForwardVector InputSocket) 1e+02))))
    (:then_1
      (LocalVariables|SetConnectorRotation (Transformation|GetWorldRotation InputSocket)))
    (:then_2
      (bind _returnvalue (Game|SpawnActorfromClass "/ConveyorBeltSystem/Blueprints/Connectors/BP_ConveyorBelt_Support_Ground_Short.BP_ConveyorBelt_Support_Ground_Short_C" (Math|Transform|MakeTransform (Math|Vector|MakeVector (.x (LocalVariables|GetConnectorLocation)) (.y (LocalVariables|GetConnectorLocation)) 0.0) (LocalVariables|GetConnectorRotation) "1.000000,1.000000,1.000000") "AlwaysSpawn" "MultiplyWithRoot" 0 0))
      (Variables|Default|SetConnector _returnvalue))))

(fn Reset
  (Utilities|FlowControl|Sequence
    (:then_0
      (Utilities|IsValid (Variables|ConveyorBeltGame|References|GetSpawnedBelt)
        (:Is%20Valid
          (Actor|DestroyActor (Variables|ConveyorBeltGame|References|GetSpawnedBelt))
          (Variables|ConveyorBeltGame|References|SetSpawnedBelt 0))))
    (:then_1
      (|CallParentFunction))))

(fn SpawnConnector
  (Utilities|IsValid (Variables|Default|GetConnector)
    (:Is%20Not%20Valid
      (Utilities|IsValid (Variables|Default|GetSelectedSocket)
        (:Is%20Valid
          (if (Class|ConveyorBeltSocket|IsAvailable (Variables|Default|GetSelectedSocket) true)
            (ConveyorBeltGame|SpawnConnectorinFrontOfSocket (Variables|Default|GetSelectedSocket))))))))