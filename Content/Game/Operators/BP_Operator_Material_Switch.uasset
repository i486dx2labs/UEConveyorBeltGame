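; Operator that switches the visual material family of all conveyor belt connectors in the level.
; On activation it confirms immediately, cycling the shared MaterialFamilyIndex on the GameMode with wraparound.
; It then applies that index's material to every ConveyorBeltConnector, choosing a material array by connector type (ground support, hatch, wall mount, distributor).
; Each connector also updates its stored original material before the parent confirm runs.
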(fn ConstructionScript
  (|CallParentFunction))

(fn OnActivate
  (|CallParentFunction)
  (CallFunction|Confirm))

(fn Confirm
  (Utilities|FlowControl|Sequence
    (:then_0
      (ConveyorBeltGame|IncreaseMaterialFamilyIndex))
    (:then_1
      (bind _outactors (Actor|GetAllActorsOfClass "/Script/ConveyorBeltSystem.ConveyorBeltConnector"))
      (for _array_element _outactors
        (ConveyorBeltGame|ApplyCurrentMaterialFamily _array_element)))
    (:then_2
      (|CallParentFunction))))

(fn IncreaseMaterialFamilyIndex
  (Variables|/Game/FirstPerson/Blueprints/BP_FirstPersonGameMode.BP_FirstPersonGameMode_C|SetMaterialFamilyIndex (Variables|Default|GetGameMode) (Math|Integer|%(Integer) (+ (Variables|/Game/FirstPerson/Blueprints/BP_FirstPersonGameMode.BP_FirstPersonGameMode_C|GetMaterialFamilyIndex (Variables|Default|GetGameMode)) 1) (Variables|ConveyorBeltGame|GetMaterialFamilyCount))))

(fn ApplyCurrentMaterialFamily
  (params (Connector :type Conveyor%20Belt%20Connector%20Object%20Reference))
  (switch Utilities|FlowControl|Switch|SwitchonEConnectorType (Variables|/Script/ConveyorBeltSystem.ConveyorBeltConnector|GetConnectorType Connector)
    (:GroundSupport
      (ConveyorBeltGame|ApplyCurrentMaterialFamilyInternal Connector (Variables|ConveyorBeltGame|GetGroundSupportMaterials)))
    (:Hatch
      (ConveyorBeltGame|ApplyCurrentMaterialFamilyInternal Connector (Variables|ConveyorBeltGame|GetHatchMaterials)))
    (:WallMount
      (ConveyorBeltGame|ApplyCurrentMaterialFamilyInternal Connector (Variables|ConveyorBeltGame|GetWallMountMaterials)))
    (:Distributor
      (ConveyorBeltGame|ApplyCurrentMaterialFamilyInternal Connector (Variables|ConveyorBeltGame|GetDistributorMaterials)))))

(fn ApplyCurrentMaterialFamilyInternal
  (params (Connector :type Conveyor%20Belt%20Connector%20Object%20Reference) (MaterialFamily :type Array%20of%20Material%20Instance%20Object%20References))
  (Class|ConveyorBeltConnector|ApplyMaterial Connector (Utilities|Array|Get(acopy) MaterialFamily (Variables|/Game/FirstPerson/Blueprints/BP_FirstPersonGameMode.BP_FirstPersonGameMode_C|GetMaterialFamilyIndex (Variables|Default|GetGameMode))))
  (Class|ConveyorBeltConnector|UpdateOriginalMaterial Connector))