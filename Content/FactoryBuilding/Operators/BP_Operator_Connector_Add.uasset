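; Factory-building operator that places a new connector, spawning a preview actor with the current material theme on activation.
; Ground and wall raycasters are queried according to the connector's placement flags; location callbacks move it, aligning it to the normal on walls.
; Increase/decrease input yaws ground connectors in 45-degree steps, or adjusts offset while Left Alt is held.
; Confirming enables collision and releases the reference, while Reset destroys any unconfirmed connector.
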(event Input|EnhancedActionEvents|EnhancedInputActionIA_Increase
  (params (ActionValue :type Boolean) (ElapsedSeconds :type Float%20%28double-precision%29) (TriggeredSeconds :type Float%20%28double-precision%29) (InputAction :type Input%20Action%20Object%20Reference :default "/Game/FactoryBuilding/Input/IA_Increase.IA_Increase"))
  (ConveyorBeltGame|Increase 1.0))

(event Input|EnhancedActionEvents|EnhancedInputActionIA_Decrease
  (params (ActionValue :type Boolean) (ElapsedSeconds :type Float%20%28double-precision%29) (TriggeredSeconds :type Float%20%28double-precision%29) (InputAction :type Input%20Action%20Object%20Reference :default "/Game/FactoryBuilding/Input/IA_Decrease.IA_Decrease"))
  (ConveyorBeltGame|Increase -1.0))

(fn ConstructionScript
  (|CallParentFunction))

(fn SpawnConnector
  (Utilities|FlowControl|Sequence
    (:then_0
      (Utilities|IsValid (Variables|ConveyorBeltGame|References|GetConnector)
        (:Is%20Not%20Valid
          (bind _returnvalue (Game|SpawnActorfromClass (Variables|ConveyorBeltGame|Settings|GetConnectorType) (Variables|Default|GetOrigin) "Undefined" "MultiplyWithRoot" 0 0))
          (Variables|ConveyorBeltGame|References|SetConnector _returnvalue))))
    (:then_1
      (Variables|/Script/ConveyorBeltSystem.ConveyorBeltConnector|SetMaterialTheme (Variables|ConveyorBeltGame|References|GetConnector) (Default|GetCurrentMaterialTheme (Variables|Default|GetGameMode)))
      (Class|ConveyorBeltConnector|ApplyMaterialTheme (Variables|ConveyorBeltGame|References|GetConnector)))))

(fn OnActivate
  (Utilities|FlowControl|Sequence
    (:then_0
      (ConveyorBeltGame|SpawnConnector))
    (:then_1
      (|CallParentFunction))))

(fn Reset
  (Utilities|FlowControl|Sequence
    (:then_0
      (Utilities|IsValid (Variables|ConveyorBeltGame|References|GetConnector)
        (:Is%20Valid
          (Actor|DestroyActor (Variables|ConveyorBeltGame|References|GetConnector)))))
    (:then_1
      (|CallParentFunction))))

(fn OnGroundLocationChanged
  (params (Location :type Vector :default "0, 0, 0"))
  (|CallParentFunction Location)
  (Transformation|SetActorLocation (Variables|ConveyorBeltGame|References|GetConnector) Location false false))

(fn OnWallLocationChanged
  (params (Location :type Vector :default "0, 0, 0") (Normal :type Vector :default "0, 0, 0"))
  (|CallParentFunction Location Normal)
  (Transformation|SetActorLocation (Variables|ConveyorBeltGame|References|GetConnector) Location false false)
  (Transformation|SetActorRotation (Variables|ConveyorBeltGame|References|GetConnector) (Math|Conversions|RotationFromXVector Normal)))

(fn Rotate
  (params (Step :type Float%20%28double-precision%29))
  (Class|Actor|AddActorWorldRotation (Variables|ConveyorBeltGame|References|GetConnector) (Math|Rotator|MakeRotator 0.0 0.0 (* Step 45.0))))

(fn IsGroundConnector
  (Utilities|IsValid (Variables|ConveyorBeltGame|References|GetConnector)
    (:Is%20Valid
      (return (Variables|/Script/ConveyorBeltSystem.ConveyorBeltConnector|GetbCanPlaceOnGround (Variables|ConveyorBeltGame|References|GetConnector))))
    (:Is%20Not%20Valid
      (return false))))

(fn IsWallConnector
  (Utilities|IsValid (Variables|ConveyorBeltGame|References|GetConnector)
    (:Is%20Valid
      (return (Variables|/Script/ConveyorBeltSystem.ConveyorBeltConnector|GetbCanPlaceOnWall (Variables|ConveyorBeltGame|References|GetConnector))))
    (:Is%20Not%20Valid
      (return false))))

(fn Increase
  (params (Step :type Float%20%28double-precision%29))
  (Utilities|IsValid (Variables|ConveyorBeltGame|References|GetConnector)
    (:Is%20Valid
      (if (ConveyorBeltGame|IsAlternateModeEnabled)
        (Class|ConveyorBeltConnector|IncrementOffset (Variables|ConveyorBeltGame|References|GetConnector) (Math|Float|Truncate Step))
        (elif (ConveyorBeltGame|IsGroundConnector)
          (ConveyorBeltGame|Rotate Step))))))

(fn QueryRaycasters
  (|CallParentFunction)
  (Utilities|FlowControl|Sequence
    (:then_0
      (if (ConveyorBeltGame|IsGroundConnector)
        (Default|Query (Variables|Default|GetGroundRaycaster) self)))
    (:then_1
      (if (ConveyorBeltGame|IsWallConnector)
        (Default|Query (Variables|Default|GetWallRaycaster) self)))))

(fn IsAlternateModeEnabled
  (return (Game|Player|IsInputKeyDown (Game|GetPlayerController 0) "LeftAlt")))

(fn ConfirmOperation
  (Utilities|FlowControl|Sequence
    (:then_0
      (Utilities|IsValid (Variables|ConveyorBeltGame|References|GetConnector)
        (:Is%20Valid
          (Class|ConveyorBeltConnector|ApplyCollisionMode (Variables|ConveyorBeltGame|References|GetConnector) "QueryAndPhysics")
          ;[0 0 0 1 12] Forget the connector otherwise it will be destroyed
          (Variables|ConveyorBeltGame|References|SetConnector 0))))
    (:then_1
      (|CallParentFunction))))