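; Factory-building operator that upgrades a single selected conveyor belt to another belt type.
; On activation it enters single-selection mode before running the parent activation.
; When a belt is picked, it looks up the new type in BeltTypeMap by the belt's segment mesh path.
; It then has the Manager's replacer swap the belt and confirms the operation, even if the lookup finds no match.
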(fn ConstructionScript
  (|CallParentFunction))

(fn OnActivate
  (Utilities|FlowControl|Sequence
    (:then_0
      (CallFunction|EnterSingleSelectionMode "NewEnumerator2"))
    (:then_1
      (|CallParentFunction))))

(fn OnBeltSelected
  (params (Belt :type Conveyor%20Belt%20Actor%20Object%20Reference))
  (bind _belttypemap (Variables|ConveyorBeltGame|References|GetBeltTypeMap))
  (bind _segmentmesh (Variables|/Script/ConveyorBeltSystem.ConveyorBeltActor|GetSegmentMesh Belt))
  (bind _returnvalue (Class|KismetSystemLibrary|ToSoftObjPath(SoftObjRef) _segmentmesh))
  (bind (_value _returnvalue_2) (Utilities|Map|Find _belttypemap _returnvalue))
  (|CallParentFunction Belt)
  (Utilities|FlowControl|Sequence
    (:then_0
      (if _returnvalue_2
        (LocalVariables|SetNewBeltType _value)))
    (:then_1
      (Class|ConveyorBeltReplacer|Replace (Class|ConveyorBeltManager|GetReplacer (Variables|Default|GetManager)) (Variables|Default|GetSelectedBelt) (LocalVariables|GetNewBeltType)))
    (:then_2
      (CallFunction|ConfirmOperation))))