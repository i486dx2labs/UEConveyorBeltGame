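; Factory-building operator for placing conveyor belts between sockets.
; Selecting an available socket spawns a short ground support connector in front of it and a belt to that connector, re-laid out as the ground location or adjustment changes.
; Hovering an available socket rebuilds the belt snapped to it, and leaving restores the ground connector.
; Confirming accepts a valid layout and sets GameMode as producer or consumer at hatch supports.
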(fn ConstructionScript
  (|CallParentFunction))

(fn OnActivate
  (Utilities|FlowControl|Sequence
    (:then_0
      (CallFunction|EnterSingleSelectionMode "NewEnumerator3"))
    (:then_1
      (Default|SetSingleTarget (Variables|Default|GetOutputSocketRaycaster) "NewEnumerator6"))
    (:then_2
      (|CallParentFunction))))

(fn OnSocketSelected
  (params (Socket :type Conveyor%20Belt%20Socket%20Object%20Reference))
  (|CallParentFunction Socket)
  (if (Class|ConveyorBeltSocket|IsAvailable Socket true)
    (CallFunction|SpawnConnector)
    (ConveyorBeltGame|SpawnBelt Socket (Class|ConveyorBeltConnector|GetSingleOutputSocket (Variables|Default|GetConnector) true))))

(fn SpawnBelt
  (params (InputSocket :type Conveyor%20Belt%20Socket%20Object%20Reference) (OutputSocket :type Conveyor%20Belt%20Socket%20Object%20Reference))
  (bind _returnvalue (Class|ConveyorBeltManager|BuildOneShotUsingSockets (Variables|Default|GetManager) InputSocket OutputSocket "/ConveyorBeltSystem/Blueprints/Belts/BP_ConveyorBelt_01.BP_ConveyorBelt_01_C" "None"))
  (bind _output_get (Variables|ConveyorBeltGame|References|SetSpawnedBelt _returnvalue))
  (Utilities|Array|Add (Variables|/Game/FactoryBuilding/Raycasters/AC_Raycaster_SelectionTarget.AC_Raycaster_SelectionTarget_C|GetIgnoredActors (Variables|Default|GetOutputSocketRaycaster)) _output_get))

(fn UpdateBeltLayout
  (Utilities|IsValid (Variables|ConveyorBeltGame|References|GetSpawnedBelt)
    (:Is%20Valid
      (Class|ConveyorBeltLayouter|Layout (Class|ConveyorBeltManager|GetLayouter (Variables|Default|GetManager)) (Variables|ConveyorBeltGame|References|GetSpawnedBelt)))))

(fn SpawnConnectorinFrontOfSocket
  (params (InputSocket :type Conveyor%20Belt%20Socket%20Object%20Reference))
  (Utilities|FlowControl|Sequence
    (:then_0
      (LocalVariables|SetConnectorLocation (+ (Transformation|GetWorldLocation InputSocket) (* (Math|Vector|GetForwardVector InputSocket) 1e+02))))
    (:then_1
      (LocalVariables|SetConnectorRotation (Transformation|GetWorldRotation InputSocket)))
    (:then_2
      (bind _returnvalue (Game|SpawnActorfromClass "/ConveyorBeltSystem/Blueprints/Connectors/BP_ConveyorBelt_Support_Ground_Short.BP_ConveyorBelt_Support_Ground_Short_C" (Math|Transform|MakeTransform (Math|Vector|MakeVector (.x (LocalVariables|GetConnectorLocation)) (.y (LocalVariables|GetConnectorLocation)) 0.0) (LocalVariables|GetConnectorRotation) "1.000000,1.000000,1.000000") "AlwaysSpawn" "MultiplyWithRoot" 0 0))
      (Variables|Default|SetConnector _returnvalue))
    (:then_3
      (Utilities|Array|Add (Variables|/Game/FactoryBuilding/Raycasters/AC_Raycaster_SelectionTarget.AC_Raycaster_SelectionTarget_C|GetIgnoredActors (Variables|Default|GetOutputSocketRaycaster)) (Variables|Default|GetConnector)))))

(fn Reset
  (Utilities|FlowControl|Sequence
    (:then_0
      (Utilities|IsValid (Variables|ConveyorBeltGame|References|GetSpawnedBelt)
        (:Is%20Valid
          (Actor|DestroyActor (Variables|ConveyorBeltGame|References|GetSpawnedBelt))
          (Variables|ConveyorBeltGame|References|SetSpawnedBelt 0))))
    (:then_1
      (Utilities|Array|Clear (Variables|/Game/FactoryBuilding/Raycasters/AC_Raycaster_SelectionTarget.AC_Raycaster_SelectionTarget_C|GetIgnoredActors (Variables|Default|GetOutputSocketRaycaster))))
    (:then_2
      (|CallParentFunction))))

(fn SpawnConnector
  (Utilities|IsValid (Variables|Default|GetConnector)
    (:Is%20Not%20Valid
      (Utilities|IsValid (Variables|Default|GetSelectedSocket)
        (:Is%20Valid
          (if (Class|ConveyorBeltSocket|IsAvailable (Variables|Default|GetSelectedSocket) true)
            (ConveyorBeltGame|SpawnConnectorinFrontOfSocket (Variables|Default|GetSelectedSocket))))))))

(fn OnGroundLocationChanged
  (params (Location :type Vector :default "0, 0, 0"))
  (|CallParentFunction Location)
  (ConveyorBeltGame|UpdateBeltLayout))

(fn Increase
  (params (Step :type Float%20%28double-precision%29))
  (|CallParentFunction Step)
  (ConveyorBeltGame|UpdateBeltLayout))

(fn ConfirmOperation
  (Utilities|FlowControl|Sequence
    (:then_0
      (Utilities|IsValid (Variables|ConveyorBeltGame|References|GetSpawnedBelt)
        (:Is%20Valid
          (if (Variables|/Script/ConveyorBeltSystem.ConveyorBeltActor|GetbValidLayout (Variables|ConveyorBeltGame|References|GetSpawnedBelt))
            (Utilities|FlowControl|Sequence
              (:then_0
                (Class|ConveyorBeltActor|AcceptLayout (Variables|ConveyorBeltGame|References|GetSpawnedBelt) "Link"))
              (:then_1
                (Utilities|Casting|CastToBP_ConveyorBelt_Support_Hatch_Out (Class|ConveyorBeltSocket|GetOwnerConnector (Variables|/Script/ConveyorBeltSystem.ConveyorBeltActor|GetInputSocket (Variables|ConveyorBeltGame|References|GetSpawnedBelt))))
                (Variables|/Script/ConveyorBeltSystem.ConveyorBeltActor|SetItemProducer (Variables|ConveyorBeltGame|References|GetSpawnedBelt) (Variables|Default|GetGameMode)))
              (:then_2
                (Utilities|Casting|CastToBP_ConveyorBelt_Support_Hatch_In (Class|ConveyorBeltSocket|GetOwnerConnector (Variables|/Script/ConveyorBeltSystem.ConveyorBeltActor|GetOutputSocket (Variables|ConveyorBeltGame|References|GetSpawnedBelt))))
                (Variables|/Script/ConveyorBeltSystem.ConveyorBeltActor|SetItemConsumer (Variables|ConveyorBeltGame|References|GetSpawnedBelt) (Variables|Default|GetGameMode)))
              (:then_3
                ;[0 0 0 1 12] Forget the belt otherwise it will be destroyed
                (Variables|ConveyorBeltGame|References|SetSpawnedBelt 0)))))))
    (:then_1
      (|CallParentFunction))))

(fn QueryRaycasters
  (|CallParentFunction)
  (Utilities|IsValid (Variables|ConveyorBeltGame|References|GetSpawnedBelt)
    (:Is%20Valid
      (Default|Query (Variables|Default|GetOutputSocketRaycaster) self))))

(fn OnSocketMouseEnter
  (params (Socket :type Conveyor%20Belt%20Socket%20Object%20Reference))
  (|CallParentFunction Socket)
  (if (and (Utilities|IsValid (Variables|ConveyorBeltGame|References|GetSpawnedBelt)) (Class|ConveyorBeltSocket|IsAvailable Socket false))
    (ConveyorBeltGame|SnapBelttoOutputSocket Socket)))

(fn SnapBelttoOutputSocket
  (params (OutputSocket :type Conveyor%20Belt%20Socket%20Object%20Reference))
  (CallFunction|Print "Snapping belt to output socket")
  (Utilities|FlowControl|Sequence
    (:then_0
      (LocalVariables|SetInputSocket (Variables|/Script/ConveyorBeltSystem.ConveyorBeltActor|GetInputSocket (Variables|ConveyorBeltGame|References|GetSpawnedBelt)))
      (Actor|DestroyActor (Variables|ConveyorBeltGame|References|GetSpawnedBelt)))
    (:then_1
      (Utilities|IsValid (Variables|Default|GetConnector)
        (:Is%20Valid
          (Actor|DestroyActor (Variables|Default|GetConnector)))))
    (:then_2
      (ConveyorBeltGame|SpawnBelt (LocalVariables|GetInputSocket) OutputSocket))))

(fn OnSocketMouseExit
  (params (Socket :type Conveyor%20Belt%20Socket%20Object%20Reference))
  (|CallParentFunction Socket)
  (Utilities|IsValid (Variables|ConveyorBeltGame|References|GetSpawnedBelt)
    (:Is%20Valid
      (if (== (Variables|/Script/ConveyorBeltSystem.ConveyorBeltActor|GetOutputSocket (Variables|ConveyorBeltGame|References|GetSpawnedBelt)) Socket)
        (ConveyorBeltGame|RestoreGroundConnector)))))

(fn RestoreGroundConnector
  (CallFunction|Print "Restoring ground connector")
  (Utilities|FlowControl|Sequence
    (:then_0
      (LocalVariables|SetInputSocket (Variables|/Script/ConveyorBeltSystem.ConveyorBeltActor|GetInputSocket (Variables|ConveyorBeltGame|References|GetSpawnedBelt)))
      (Actor|DestroyActor (Variables|ConveyorBeltGame|References|GetSpawnedBelt)))
    (:then_1
      ;[0 0 0 1 12] Simulate the input socket selection so that we restart the operation
      (CallFunction|OnSocketSelected (LocalVariables|GetInputSocket)))))