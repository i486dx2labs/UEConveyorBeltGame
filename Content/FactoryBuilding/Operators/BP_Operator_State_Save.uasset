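; Factory-building operator state that saves the game's world state.
; It confirms itself as soon as it activates, then constructs a BP_SaveGame from the world state supplied by the Manager's serializer.
; Confirmation writes that object to the default save slot, prints a notice and hands off to the parent confirm logic.
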(event EventBeginPlay
  (|CallParentFunction) ; This node is disabled and will not be called.\nDrag off pins to build functionality.
)

(event Collision|EventActorBeginOverlap
  (params (OtherActor :type Actor%20Object%20Reference)))

(event EventTick
  (params (DeltaSeconds :type Float%20%28single-precision%29)))

(fn ConstructionScript
  (|CallParentFunction))

(fn OnActivate
  (|CallParentFunction)
  (CallFunction|Confirm))

(fn ConfirmOperation
  (bind _savegame (ConveyorBeltGame|CreateSaveGame))
  (SaveGame|SaveGametoSlot _savegame "Default")
  (CallFunction|Print "Game state saved")
  (|CallParentFunction))

(fn CreateSaveGame
  (bind _returnvalue (Game|ConstructObjectfromClass "/Game/FactoryBuilding/State/BP_SaveGame.BP_SaveGame_C" (Class|ConveyorBeltSerializer|GetWorldState (Class|ConveyorBeltManager|GetSerializer (Variables|Default|GetManager)))))
  (return _returnvalue))