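; Dismantle operator for the factory building system that deletes connectors and belts the player selects.
; Activation enters selection mode before running the parent operator logic.
; A selected connector is destroyed and the operation confirmed; a selected belt first has every item actor riding on it destroyed, then the belt itself, then confirms.
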(fn ConstructionScript
  (|CallParentFunction))

(fn OnActivate
  (CallFunction|EnterSelectionMode (LocalVariables|GetTargets))
  (|CallParentFunction))

(fn OnConnectorSelected
  (params (Connector :type Conveyor%20Belt%20Connector%20Object%20Reference))
  (|CallParentFunction Connector)
  (Actor|DestroyActor (Variables|Default|GetSelectedConnector))
  (CallFunction|ConfirmOperation))

(fn OnBeltSelected
  (params (Belt :type Conveyor%20Belt%20Actor%20Object%20Reference))
  (|CallParentFunction Belt)
  (Utilities|FlowControl|Sequence
    (:then_0
      (for _array_element (Variables|/Script/ConveyorBeltSystem.ConveyorBeltActor|GetItems (Variables|Default|GetSelectedBelt))
        (Actor|DestroyActor (.Actor (Utilities|Struct|BreakConveyorBeltItem _array_element)))))
    (:then_1
      (Actor|DestroyActor (Variables|Default|GetSelectedBelt)))
    (:then_2
      (CallFunction|ConfirmOperation))))