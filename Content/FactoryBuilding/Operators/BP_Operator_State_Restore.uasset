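; BP_Operator_State_Restore is a factory-building operator that restores the saved game state.
; Activating it confirms immediately, with no extra input step.
; On confirmation it loads the BP_SaveGame from the default slot, stopping if the cast fails, and passes its WorldState to the Manager's serializer to restore the world.
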(event EventBeginPlay
  (|CallParentFunction) ; This node is disabled and will not be called.\nDrag off pins to build functionality.
)

(event Collision|EventActorBeginOverlap
  (params (OtherActor :type Actor%20Object%20Reference)))

(event EventTick
  (params (DeltaSeconds :type Float%20%28single-precision%29)))

(fn ConstructionScript
  (|CallParentFunction))

(fn OnActivate
  (|CallParentFunction)
  (CallFunction|Confirm))

(fn ConfirmOperation
  (bind _returnvalue (SaveGame|LoadGamefromSlot "Default"))
  (bind _asbp_save_game (Utilities|Casting|CastToBP_SaveGame _returnvalue))
  (ConveyorBeltGame|LoadSaveGame _asbp_save_game)
  (CallFunction|Print "Game state restored")
  (|CallParentFunction))

(fn LoadSaveGame
  (params (SaveGame :type BP%20Save%20Game%20Object%20Reference))
  (Class|ConveyorBeltSerializer|RestoreWorldState (Class|ConveyorBeltManager|GetSerializer (Variables|Default|GetManager)) (Variables|/Game/FactoryBuilding/State/BP_SaveGame.BP_SaveGame_C|GetWorldState SaveGame)))