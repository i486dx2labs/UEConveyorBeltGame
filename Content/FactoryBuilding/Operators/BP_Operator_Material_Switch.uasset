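; Operator Blueprint that switches the conveyor belt material theme in the factory building game.
; Activating it confirms immediately, with no further input step.
; Confirmation increments the GameMode's theme index, then pushes the current theme to every ConveyorBeltConnector in the level and re-applies its materials before running the parent confirm.
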(fn ConstructionScript
  (|CallParentFunction))

(fn OnActivate
  (|CallParentFunction)
  (CallFunction|Confirm))

(fn AdvanceMaterialTheme
  (Variables|/Game/FirstPerson/Blueprints/BP_FirstPersonGameMode.BP_FirstPersonGameMode_C|SetMaterialThemeIndex (Variables|Default|GetGameMode) (+ (Variables|/Game/FirstPerson/Blueprints/BP_FirstPersonGameMode.BP_FirstPersonGameMode_C|GetMaterialThemeIndex (Variables|Default|GetGameMode)) 1)))

(fn ApplyMaterialTheme
  (params (Connector :type Conveyor%20Belt%20Connector%20Object%20Reference))
  (Variables|/Script/ConveyorBeltSystem.ConveyorBeltConnector|SetMaterialTheme Connector (Default|GetCurrentMaterialTheme (Variables|Default|GetGameMode)))
  (Class|ConveyorBeltConnector|ApplyMaterialTheme Connector))

(fn ConfirmOperation
  (Utilities|FlowControl|Sequence
    (:then_0
      (ConveyorBeltGame|AdvanceMaterialTheme))
    (:then_1
      (bind _outactors (Actor|GetAllActorsOfClass "/Script/ConveyorBeltSystem.ConveyorBeltConnector"))
      (for _array_element _outactors
        (ConveyorBeltGame|ApplyMaterialTheme _array_element)))
    (:then_2
      (|CallParentFunction))))