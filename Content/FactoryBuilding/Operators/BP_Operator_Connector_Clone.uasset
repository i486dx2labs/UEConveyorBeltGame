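; Connector operator for factory building that clones a selected connector.
; On activation it enters single selection mode, then spawns an actor of the selected connector's class at the same transform and copies its offset.
; It then spawns a BP_Operator_Connector_Add with the clone as its connector and has the GameMode activate it, handing over to the add operator.
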(fn ConstructionScript
  (|CallParentFunction))

(fn OnConnectorSelected
  (params (Connector :type Conveyor%20Belt%20Connector%20Object%20Reference))
  (|CallParentFunction Connector)
  (Utilities|FlowControl|Sequence
    (:then_0
      (bind _returnvalue (Game|SpawnActorfromClass (Utilities|GetClass Connector) (Transformation|GetActorTransform Connector) "AlwaysSpawn" "MultiplyWithRoot" 0 0))
      (LocalVariables|SetClone _returnvalue))
    (:then_1
      (Class|ConveyorBeltConnector|SetOffset (LocalVariables|GetClone) (Variables|/Script/ConveyorBeltSystem.ConveyorBeltConnector|GetOffset Connector)))
    (:then_2
      (bind _returnvalue_2 (Game|SpawnActorfromClass "/Game/FactoryBuilding/Operators/BP_Operator_Connector_Add.BP_Operator_Connector_Add_C" (Variables|Default|GetOrigin) "AlwaysSpawn" "MultiplyWithRoot" 0 0 (LocalVariables|GetClone) 0 0))
      (Default|ActivateOperator (Variables|Default|GetGameMode) _returnvalue_2))))

(fn OnActivate
  (Utilities|FlowControl|Sequence
    (:then_0
      (CallFunction|EnterSingleSelectionMode "NewEnumerator0"))
    (:then_1
      (|CallParentFunction))))