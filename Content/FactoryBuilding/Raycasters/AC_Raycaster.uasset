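; AC_Raycaster is a raycasting component for factory building that provides camera-based trace points and an empty Query function.
; The trace starts at the first player's camera manager location and extends along its forward vector by Distance.
; On BeginPlay it caches the game mode as BP_FirstPersonGameMode.
; Query takes an Operator but has no logic here, and no trace is performed in this asset.
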(event EventBeginPlay
  (ConveyorBeltGame|FindGameMode))

(fn Query
  (params (Operator :type BP%20Operator%20Object%20Reference)))

(fn GetTraceStart
  (return (Camera|GetCameraLocation (Variables|/Script/Engine.PlayerController|GetPlayerCameraManager (Game|GetPlayerController 0)))))

(fn GetTraceEnd
  (return (+ (ConveyorBeltGame|GetTraceStart) (* (Transformation|GetActorForwardVector (Variables|/Script/Engine.PlayerController|GetPlayerCameraManager (Game|GetPlayerController 0))) (Variables|ConveyorBeltGame|GetDistance)))))

(fn FindGameMode
  (bind _asbp_first_person_game_mode (Utilities|Casting|CastToBP_FirstPersonGameMode (Game|GetGameMode)))
  (Variables|ConveyorBeltGame|SetGameMode _asbp_first_person_game_mode))