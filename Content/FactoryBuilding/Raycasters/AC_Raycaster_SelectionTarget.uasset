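; Raycaster component for factory building that finds which selection target the trace hits and reports it to the querying operator.
; Query multi-traces the Camera channel, skipping ignored actors, and offers each hit to the validators of the active Targets until one handles it, else signals nothing hovered.
; Validators are lazily constructed from a target-type-to-class map, with a default fallback.
; The per-type connector, socket and belt handlers are disconnected stubs.
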(fn Query
  (params (Operator :type BP%20Operator%20Object%20Reference))
  (|CallParentFunction Operator)
  (bind (_outhits _returnvalue) (Collision|MultiLineTraceByChannel (CallFunction|GetTraceStart) (CallFunction|GetTraceEnd) "TraceTypeQuery2" false (Variables|ConveyorBeltGame|GetIgnoredActors) "None"))
  (if _returnvalue
    (for _array_element _outhits
      (bind _handled (ConveyorBeltGame|HandleSomethingHit Operator _array_element))
      (if _handled
        (return))))
  (ConveyorBeltGame|HandleEmptyHit Operator))

(fn HandleSomethingHit
  (params (Operator :type BP%20Operator%20Object%20Reference) (Hit :type Hit%20Result%20Structure))
  (bind (_bblockinghit _binitialoverlap _time _distance _location _impactpoint _normal _impactnormal _physmat _hitactor _hitcomponent) (Collision|BreakHitResult Hit))
  (bind _handled (ConveyorBeltGame|HandleActorHit Operator _hitactor _hitcomponent))
  (return _handled))

(fn HandleActorHit
  (params (Operator :type BP%20Operator%20Object%20Reference) (Actor :type Actor%20Object%20Reference) (Component :type Primitive%20Component%20Object%20Reference))
  (for _array_element (Variables|ConveyorBeltGame|GetTargets)
    (bind _validator (ConveyorBeltGame|GetValidator _array_element))
    (bind _handled (Default|HandleSelectionTarget _validator Operator Actor Component))
    (if _handled
      (return true)))
  (return false))

(fn HandleEmptyHit
  (params (Operator :type BP%20Operator%20Object%20Reference))
  (Default|OnNothingHovered Operator))

(fn HandleConnectorTarget
  (params (Operator :type BP%20Operator%20Object%20Reference) (Actor :type Actor%20Object%20Reference)))

(fn HandleGroundConnectorTarget
  (params (Operator :type BP%20Operator%20Object%20Reference) (Actor :type Actor%20Object%20Reference)))

(fn HandleInputSocketTarget
  (params (Operator :type BP%20Operator%20Object%20Reference) (Actor :type Actor%20Object%20Reference) (Hit :type Hit%20Result%20Structure)))

(fn HandleOutputSocketTarget
  (params (Operator :type BP%20Operator%20Object%20Reference) (Actor :type Actor%20Object%20Reference) (Hit :type Hit%20Result%20Structure)))

(fn HandleBeltTarget
  (params (Operator :type BP%20Operator%20Object%20Reference) (Actor :type Actor%20Object%20Reference)))

(fn SetSingleTarget
  (params (Target :type E_SelectionTarget%20Enum :default "NewEnumerator0"))
  (Variables|ConveyorBeltGame|SetTargets (Utilities|Array|MakeArray Target)))

(fn InitValidators
  (Utilities|FlowControl|Sequence
    (:then_0
      (bind _returnvalue (Game|ConstructObjectfromClass "/Game/FactoryBuilding/Raycasters/O_SelectionTargetValidator.O_SelectionTargetValidator_C"))
      (Variables|ConveyorBeltGame|SetDefaultValidator _returnvalue))
    (:then_1
      (if (Utilities|Map|IsEmpty (Variables|ConveyorBeltGame|GetTargetValidators))
        (bind _keys (Utilities|Map|Keys (Variables|ConveyorBeltGame|GetTargetValidatorTypes)))
        (for _array_element _keys
          (bind _returnvalue_2 (Game|ConstructObjectfromClass (.Value (Utilities|Map|Find (Variables|ConveyorBeltGame|GetTargetValidatorTypes) _array_element))))
          (Utilities|Map|Add (Variables|ConveyorBeltGame|GetTargetValidators) _array_element _returnvalue_2))))))

(fn GetValidator
  (params (SelectionTarget :type E_SelectionTarget%20Enum :default "NewEnumerator0"))
  (bind _targetvalidators (Variables|ConveyorBeltGame|GetTargetValidators))
  (bind (_value _returnvalue) (Utilities|Map|Find _targetvalidators SelectionTarget))
  (Utilities|FlowControl|Sequence
    (:then_0
      (Utilities|IsValid (Variables|ConveyorBeltGame|GetDefaultValidator)
        (:Is%20Not%20Valid
          (ConveyorBeltGame|InitValidators))))
    (:then_1
      (if _returnvalue
        (return _value)
        (else
          (Development|PrintText (Utilities|Text|FormatText "No validator found for type: {type}" (Utilities|String|EnumtoString SelectionTarget)))
          (return (Variables|ConveyorBeltGame|GetDefaultValidator)))))))

(fn IgnoreActor
  (params (Actor :type Actor%20Object%20Reference))
  (Utilities|Array|AddUnique (Variables|ConveyorBeltGame|GetIgnoredActors) Actor))

(fn ClearIgnoredActors
  (Utilities|Array|Clear (Variables|ConveyorBeltGame|GetIgnoredActors)))